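; Box001_Blueprint is a trigger-box light switch that lets the player toggle a spotlight while standing inside it.
; Box overlap begin and end set Inbox, enable or disable input from player controller 0, and show or hide the Presslight prompt component to match.
; The lights input action flips the Lightoff flag and toggles visibility of the SpotLightComponent on the referenced Mylight actor.
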(event OnComponentBeginOverlap(Box)
  (params (OverlappedComponent :type Primitive%20Component%20Object%20Reference) (OtherActor :type Actor%20Object%20Reference) (OtherComp :type Primitive%20Component%20Object%20Reference) (OtherBodyIndex :type Integer) (bFromSweep :type Boolean) (SweepResult :type Hit%20Result%20Structure%20%28by%20ref%29))
  (Variables|Default|Setinbox true)
  (Input|EnableInput (Game|GetPlayerController 0))
  (Rendering|SetVisibility (Variables|Default|Getpresslight) (Variables|Default|Getinbox) false))

(event OnComponentEndOverlap(Box)
  (params (OverlappedComponent :type Primitive%20Component%20Object%20Reference) (OtherActor :type Actor%20Object%20Reference) (OtherComp :type Primitive%20Component%20Object%20Reference) (OtherBodyIndex :type Integer))
  (Variables|Default|Setinbox false)
  (Input|DisableInput (Game|GetPlayerController 0))
  (Rendering|SetVisibility (Variables|Default|Getpresslight) (Variables|Default|Getinbox) false))

(event EventBeginPlay)

(event Collision|EventActorBeginOverlap
  (params (OtherActor :type Actor%20Object%20Reference)))

(event EventTick
  (params (DeltaSeconds :type Float%20%28single-precision%29)))

(event Input|ActionEvents|InputActionlights
  (params (Key :type Key%20Structure :default "None"))
  (:Pressed
    (Variables|Default|Setlightoff (not (Variables|Default|Getlightoff)))
    (Rendering|ToggleVisibility (Variables|/Script/Engine.SpotLight|GetSpotLightComponent (Variables|Default|Getmylight)) false)))

(fn ConstructionScript)